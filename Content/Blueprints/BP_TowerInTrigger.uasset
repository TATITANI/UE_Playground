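; BP_TowerInTrigger is a trigger actor that toggles a Data Layer when the player's pawn overlaps it, apparently for entering a tower.
; On overlap it reads the runtime state of its InDataLayer, setting Unloaded or Loaded to Activated and Activated back to Loaded, non-recursively.
; Overlaps by any other actor only print a failure message.
; The OnTrigger function is an empty stub.
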(event Collision|EventActorBeginOverlap
  (params (OtherActor :type Actor%20Object%20Reference))
  (bind _returnvalue (WorldSubsystems|GetDataLayerSubsystem))
  (bind _in_data_layer (Variables|Default|GetIn%20Data%20Layer))
  (if (== OtherActor (Pawn|GetControlledPawn (Game|GetPlayerController 0)))
    (switch Utilities|FlowControl|Switch|SwitchonEDataLayerRuntimeState (Class|DataLayerSubsystem|GetDataLayerRuntimeState _returnvalue _in_data_layer)
      (:Unloaded
        (DataLayers|SetDataLayerRuntimeState _returnvalue _in_data_layer "Activated" false :!class /Script/Engine.DataLayerSubsystem :!label _label))
      (:Loaded
        (goto _label))
      (:Activated
        (DataLayers|SetDataLayerRuntimeState _returnvalue _in_data_layer "Loaded" false :!class /Script/Engine.DataLayerSubsystem)))
    (else
      (Development|PrintText "TowerIn Trigger fail"))))

(fn ConstructionScript)

(fn OnTrigger)