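; Protagonist character Blueprint that drives the CameraBoom spring arm for weapon-based aiming and slash zoom effects.
; AimCambyWeapon plays a timeline forward for GUN and reverses it for None, SWORD or BOMB, blending arm length and socket offset.
; ZoomonSlash restarts a separate ZoomInOut timeline that animates only the arm length.
; BeginPlay, Tick, overlap and the construction script are empty.
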(event EventBeginPlay)

(event Collision|EventActorBeginOverlap
  (params (OtherActor :type Actor%20Object%20Reference)))

(event EventTick
  (params (DeltaSeconds :type Float%20%28single-precision%29)))

(event EventAimCambyWeapon
  (params (WeaponType :type EWeaponType%20Enum :default "WEAPON_None"))
  (bind _cameraboom (Variables|Default|GetCameraBoom))
  (switch Utilities|FlowControl|Switch|SwitchonEWeaponType WeaponType
    (:WEAPON_None
      (if true :!label _label
        (bind (_direction _armlength _socketoffset) (Timeline|타임라인 Reverse)
          (:Update
            (Variables|/Script/Engine.SpringArmComponent|SetTargetArmLength _cameraboom _armlength)
            (Variables|/Script/Engine.SpringArmComponent|SetSocketOffset _cameraboom _socketoffset)))))
    (:SWORD
      (goto _label))
    (:GUN
      (if true
        (Timeline|타임라인 Play)))
    (:BOMB
      (goto _label))))

(event EventZoomonSlash
  (bind _armlength (Timeline|ZoomInOut PlayFromStart)
    (:Update
      (Variables|/Script/Engine.SpringArmComponent|SetTargetArmLength (Variables|Default|GetCameraBoom) _armlength))))

(fn ConstructionScript)