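; BP_FloatingDamage is a floating damage number that displays a damage value through a WBP_FloatingTxt widget in its WidgetComponent.
; On BeginPlay it caches that widget and derives MovingDuration from the time left in the widget's Fade animation, printing an error if the cast fails.
; SetDamageTxt writes the damage as integer text into the widget's TXTBody.
; The graph only stores MovingDuration and contains no movement logic.
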(event EventBeginPlay
  (bind _aswbp_floating_txt (Utilities|Casting|CastToWBP_FloatingTxt (UserInterface|GetUserWidgetObject (Variables|Default|GetWidgetComponent)))
    (:then
      (bind _output_get (Variables|Default|SetWBP%20Flating%20Txt _aswbp_floating_txt))
      (Variables|Default|SetMovingDuration (- (Class|WidgetAnimation|GetEndTime (Variables|/Game/UI/WBP_FloatingTxt.WBP_FloatingTxt_C|GetFade _output_get)) (Class|UserWidget|GetAnimationCurrentTime _output_get (Variables|/Game/UI/WBP_FloatingTxt.WBP_FloatingTxt_C|GetFade _output_get)))))
    (:CastFailed
      (Development|PrintString "WBP_FloatingTxt cast Failed" false true "(R=0.000000,G=0.660000,B=1.000000,A=1.000000)" 2.0 "Error"))))

(event EventTick
  (params (DeltaSeconds :type Float%20%28single-precision%29)))

(event EventSetDamageTxt
  (params (Damage :type Integer%20%28by%20ref%29))
  (Rendering|Components|TextRender|SetText (Variables|/Game/UI/WBP_FloatingTxt.WBP_FloatingTxt_C|GetTXT_Body (Variables|Default|GetWBP%20Flating%20Txt)) (Utilities|Text|ToText(Integer) Damage)))

(fn ConstructionScript)